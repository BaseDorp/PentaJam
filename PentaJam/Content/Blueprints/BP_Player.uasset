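; Player Blueprint that handles health, enemy contact damage, respawning and temporary immunity.
; Collider overlaps with an actor displayed as BP_EnemyCharacter subtract health, then grant brief immunity through a Delay.
; Tick teleports the player to a fixed point and grants immunity at zero health, but Respawn never restores Health, so this repeats every frame.
; Ammo reload and bounce-back impulse logic are unconnected and never run.
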(event OnComponentBeginOverlap(Collider)
  (params (OverlappedComponent :type Primitive%20Component%20Object%20Reference) (OtherActor :type Actor%20Object%20Reference) (OtherComp :type Primitive%20Component%20Object%20Reference) (OtherBodyIndex :type Integer) (bFromSweep :type Boolean) (SweepResult :type Hit%20Result%20Structure%20%28by%20ref%29))
  ;[1 1 1] Enemy Collision Detection
  (if (Utilities|Enum|Equal(Enum) (Utilities|GetDisplayName OtherActor) "BP_EnemyCharacter")
    (if (not (Variables|Default|GetbIsImmune))
      (Variables|Default|Sethealth (- (Variables|Default|Gethealth) 1e+01))
      (Development|PrintString (Utilities|String|ToString(Float) (Variables|Default|Gethealth)))
      (Variables|Default|SetbIsImmune true)
      (Utilities|FlowControl|Delay 2.0)
      (Variables|Default|SetbIsImmune false))))

(event Custom|Respawn
  (Transformation|SetActorLocation "0,0.000000,220.000000" false false)
  (Development|PrintString "Hello"))

(event EventBeginPlay
  (Variables|Default|Sethealth 2e+01))

(event Collision|EventActorBeginOverlap
  (params (OtherActor :type Actor%20Object%20Reference)))

(event EventTick
  (params (DeltaSeconds :type Float%20%28single-precision%29))
  (if (<= (Variables|Default|Gethealth) 0.0)
    (Development|PrintString "died")
    (CallFunction|Respawn)
    (Variables|Default|SetbIsImmune true)
    (Utilities|FlowControl|Delay 3.0)
    (Variables|Default|SetbIsImmune false)))

(fn ConstructionScript)