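; Candle manager that lights five child-actor candles in sequence and tells the player when all are lit.
; The construction script builds the candle array, and BeginPlay sets NextCandle to the candle at the lit count, or the following one if that is already lit.
; LightNextCandle lights the current candle, increments the count and advances NextCandle.
; Tick polls the count and sets AllCandlesLit on BP_Player once it reaches five.
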(event EventBeginPlay
  (bind _ascandle (Utilities|Casting|CastToCandle (Variables|/Script/Engine.ChildActorComponent|GetChildActor (Utilities|Array|Get(acopy) (Variables|Default|GetCandlesArray) (Variables|Default|GetLitCandles)))))
  (if (Variables|/Game/Blueprints/Candle.Candle_C|GetbisLit _ascandle)
    (bind _ascandle_2 (Utilities|Casting|CastToCandle (Variables|/Script/Engine.ChildActorComponent|GetChildActor (Utilities|Array|Get(acopy) (Variables|Default|GetCandlesArray) (+ (Variables|Default|GetLitCandles) 1)))))
    (Variables|Default|SetnextCandle _ascandle_2)
    (else
      (Variables|Default|SetnextCandle _ascandle))))

(event EventTick
  (params (DeltaSeconds :type Float%20%28single-precision%29))
  (if (>= (Variables|Default|GetLitCandles) 5)
    (bind _asbp_player (Utilities|Casting|CastToBP_Player (Game|Player|GetPlayerPawn 0)))
    (Variables|/Game/Blueprints/BP_Player.BP_Player_C|SetbAllCandlesLit _asbp_player true)))

(fn ConstructionScript
  (Variables|Default|SetCandlesArray (Utilities|Array|MakeArray (Variables|Default|GetChildActor_Candle1) (Variables|Default|GetChildActor_Candle2) (Variables|Default|GetChildActor_Candle3) (Variables|Default|GetChildActor_Candle4) (Variables|Default|GetChildActor_Candle5))))

(fn LightNextCandle
  (bind _candlesarray (Variables|Default|GetCandlesArray))
  (if (not (>= (Variables|Default|GetLitCandles) 5)) ; Check if all candles are lit
    (bind _ascandle (Utilities|Casting|CastToCandle (Variables|/Script/Engine.ChildActorComponent|GetChildActor (Utilities|Array|Get(acopy) _candlesarray (Variables|Default|GetLitCandles)))))
    (Default|SetCandleLight _ascandle true)
    (bind _output_get (Variables|Default|SetLitCandles (+ (Variables|Default|GetLitCandles) 1)))
    (bind _ascandle_2 (Utilities|Casting|CastToCandle (Variables|/Script/Engine.ChildActorComponent|GetChildActor (Utilities|Array|Get(acopy) _candlesarray _output_get))))
    (Variables|Default|SetnextCandle _ascandle_2)))