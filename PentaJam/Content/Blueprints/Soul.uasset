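; Soul actor that drifts toward the next candle tracked by its Candle Manager and lights it on arrival.
; Each tick it interpolates its location toward the manager's NextCandle.
; Once within a small tolerance, it tells the manager to light that candle and destroys itself.
; The manager reference is exposed on spawn, so the spawner supplies it.
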(event EventBeginPlay)

(event EventTick
  (params (DeltaSeconds :type Float%20%28single-precision%29))
  (bind _candlemanagerreference (Variables|Default|GetCandleManagerReference))
  (bind _defaultsceneroot (Variables|Default|GetDefaultSceneRoot))
  (bind _returnvalue (Transformation|GetWorldLocation _defaultsceneroot))
  (bind _nextcandle (Variables|/Game/Blueprints/Candle_Manager.Candle_Manager_C|GetnextCandle _candlemanagerreference))
  (bind _returnvalue_2 (Transformation|GetActorLocation _nextcandle))
  (Transformation|SetActorLocation (Math|Interpolation|VInterpTo _returnvalue _returnvalue_2 DeltaSeconds 1.0) false false)
  (if (Math|Vector|Equal(Vector) _returnvalue _returnvalue_2 1e+01)
    ;[1 0 0] Note to Sam:
    ; When spawning the Soul BP, make sure to set the CandleManagerReference.
    ; I exposed the variable as a pin on spawn.
    (Default|LightNextCandle _candlemanagerreference)
    (Actor|DestroyActor)))

(fn ConstructionScript)