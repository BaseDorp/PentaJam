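; BP_BossSpawner is an actor that spawns the BP_EnemyBoss once the player has lit all candles.
; Each tick, until the boss has spawned, it casts the player pawn to BP_Player and polls its AllCandlesLit flag.
; When the flag is true, it spawns the boss at its own transform and sets BossSpawned so it only happens once.
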(event EventBeginPlay
  (|CallParentFunction) ; This node is disabled and will not be called.\nDrag off pins to build functionality.
)

(event Collision|EventActorBeginOverlap
  (params (OtherActor :type Actor%20Object%20Reference))
  (|CallParentFunction OtherActor) ; This node is disabled and will not be called.\nDrag off pins to build functionality.
)

(event EventTick
  (params (DeltaSeconds :type Float%20%28single-precision%29))
  (if (not (Variables|Default|GetbossSpawned))
    (bind _asbp_player (Utilities|Casting|CastToBP_Player (Game|Player|GetPlayerPawn 0)))
    (if (Variables|/Game/Blueprints/BP_Player.BP_Player_C|GetbAllCandlesLit _asbp_player)
      (Game|SpawnActorfromClass "/Game/Blueprints/BP_EnemyBoss.BP_EnemyBoss_C" (Transformation|GetActorTransform) "Undefined" 0 0)
      (Variables|Default|SetbossSpawned true))))

(fn ConstructionScript
  (|CallParentFunction))