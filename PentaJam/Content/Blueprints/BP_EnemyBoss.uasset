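; Boss enemy that pursues the player and loads GameLevel when killed.
; From BeginPlay, the Chase event runs AI MoveTo toward the player pawn and re-issues itself only on success, with no handling for failure.
; Sphere overlaps with actors tagged "projectile" decrement Health, and at zero or below the boss opens the level and destroys itself.
; The separate ChasePlayer function is an empty stub.
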(event OnComponentBeginOverlap(Sphere)
  (params (OverlappedComponent :type Primitive%20Component%20Object%20Reference) (OtherActor :type Actor%20Object%20Reference) (OtherComp :type Primitive%20Component%20Object%20Reference) (OtherBodyIndex :type Integer) (bFromSweep :type Boolean) (SweepResult :type Hit%20Result%20Structure%20%28by%20ref%29))
  ;[1 1 1] Collision with Bullet
  (if (Actor|ActorHasTag OtherActor "projectile")
    (Variables|Default|Sethealth (- (Variables|Default|Gethealth) 1.0))
    (if (<= (Variables|Default|Gethealth) 0.0)
      (Game|OpenLevel(byName) "GameLevel")
      (Actor|DestroyActor))))

(event Custom|Chase
  ;[1 1 1] Enemy chase player
  (AI|AIMoveTo (Class|CharacterMovementComponent|GetCharacterOwner (Variables|Character|GetCharacterMovement)) "0, 0, 0" (Game|Player|GetPlayerPawn 0) 1.0 false
    (:OnSuccess
      (CallFunction|Chase))))

(event EventBeginPlay
  (CallFunction|Chase))

(fn ConstructionScript)

(fn ChasePlayer)